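; One_Way_Platform is a side-scroller platform that characters can pass through, becoming solid only while something overlaps its Solid trigger.
; The construction script disables Platform collision and creates a dynamic material, and overlap begin and end on Solid toggle that collision.
; On the first landing hit, it turns the material and BlueLight green and calls TouchPlatform on the SideScrollerCharacter, with Counter guarding against repeats.
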(event `self.Solid.OnComponentBeginOverlap`
  (params (OtherActor :type "Actor Object Reference") (OtherComp :type "PrimitiveComponent Object Reference") (OtherBodyIndex :type Integer) (bFromSweep :type Boolean) (SweepResult :type "HitResult Structure (by ref)"))
  (`PrimitiveComponent.SetCollisionEnabled` (`self.Platform`) "QueryAndPhysics"))

(event `self.Solid.OnComponentEndOverlap`
  (params (OtherActor :type "Actor Object Reference") (OtherComp :type "PrimitiveComponent Object Reference") (OtherBodyIndex :type Integer))
  (`PrimitiveComponent.SetCollisionEnabled` (`self.Platform`) "NoCollision"))

(event `self.Platform.OnComponentHit`
  (params (OtherActor :type "Actor Object Reference") (OtherComp :type "PrimitiveComponent Object Reference") (NormalImpulse :type "Vector Structure") (Hit :type "HitResult Structure (by ref)"))
  (if (`self.Counter`)
    (`KismetSystemLibrary.PrintText` "Land2")
    (else
      (`MaterialInstanceDynamic.SetVectorParameterValue` (`self.Dynamic Material`) "Light" (struct :`G` 0.92 :`B` 0.064641 :`A` 1.0))
      (`LightComponent.SetLightColor` (`self.Blue Light`) (struct :`G` 1.0 :`B` 0.009654 :`A` 1.0) true)
      (bind _asside_scroller_character (cast `/Game/SideScrollerBP/Blueprints/SideScrollerCharacter` OtherActor))
      (`/Game/SideScrollerBP/Blueprints/SideScrollerCharacter.Touch Platform` _asside_scroller_character)
      (`KismetSystemLibrary.PrintText` "Land")
      (set `self.Counter` true))))

(fn `UserConstructionScript`
  (bind _platform (`self.Platform`))
  (`|ExecutionSequence`
    (:`then_0`
      (`PrimitiveComponent.SetCollisionEnabled` _platform "NoCollision"))
    (:`then_1`
      (bind _returnvalue (`PrimitiveComponent.CreateDynamicMaterialInstance` _platform 2 null))
      (set `self.Dynamic Material` _returnvalue))))